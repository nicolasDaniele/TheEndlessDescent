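; GA_HitReact is a gameplay ability that plays a hit reaction on its avatar.
; It gets the montage from the avatar's CombatInterface, then applies GE_HitReact and disables the character mesh's collision while it plays.
; The ability ends on montage completion only, and ending it removes the effect by its stored handle and restores the mesh to query-only collision.
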(event Custom|SetAvatarCollisionEnabled
  (params (Enabled :type Boolean))
  (Utilities|FlowControl|Sequence
    (:then_0
      (Variables|Default|GetAvatarCharacter
        (:then)
        (:else
          (bind _ascharacter (Utilities|Casting|CastToCharacter (Ability|GetAvatarActorfromActorInfo)))
          (Variables|Default|SetAvatarCharacter _ascharacter))))
    (:then_1
      (if Enabled
        (Collision|SetCollisionEnabled (Variables|/Script/Engine.Character|GetMesh (Variables|Default|GetAvatarCharacter)) "QueryOnly")
        (else
          (Collision|SetCollisionEnabled (Variables|/Script/Engine.Character|GetMesh (Variables|Default|GetAvatarCharacter)) "NoCollision"))))))

(event Ability|EventActivateAbility
  (bind _ascombat_interface (Utilities|Casting|CastToCombatInterface (Ability|GetAvatarActorfromActorInfo)))
  (bind _returnvalue (Class|CombatInterface|GetHitReactMontage _ascombat_interface))
  (|PlayMontageandWaitProxy "None" _returnvalue 1.0 "None" true 1.0 0.0 false
    (:then
      (CallFunction|SetAvatarCollisionEnabled false)
      (bind _returnvalue_2 (Ability|ApplyGameplayEffectToOwner "/Game/Blueprints/AbilitySystem/GameplayEffects/GE_HitReact.GE_HitReact_C"))
      (Variables|Default|SetActiveGE_HitReact _returnvalue_2))
    (:OnCompleted
      (Ability|EndAbility))))

(event Ability|EventOnEndAbility
  (params (bWasCancelled :type Boolean))
  (Ability|RemoveGameplayEffectFromOwnerWithHandle (Variables|Default|GetActiveGE_HitReact))
  (CallFunction|SetAvatarCollisionEnabled true))